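; BP_Ground is a road segment that populates itself with obstacles and extends the road by chaining copies of itself.
; On BeginPlay it caches arrow component transforms, shuffles them and spawns one to three BP_Obstacle actors slightly above those points.
; A short one-shot timer then spawns the next BP_Ground, offset along world X by the scaled plane size, so each segment creates its successor without limit.
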(event Custom|Event%20SpawnNextRoad
  (CallFunction|SpawnNextRoadScript))

(event EventBeginPlay
  (Utilities|FlowControl|Sequence
    (:then_0
      (CallFunction|SetSpawnPoints)
      (CallFunction|ItemsSpawn))
    (:then_1
      (Utilities|Time|SetTimerbyEvent (delegate Custom|Event%20SpawnNextRoad) 0.2))))

(fn ConstructionScript)

(fn SpawnNextRoadScript
  (bind _returnvalue (Transformation|GetActorTransform))
  (bind (_location _rotation _scale) (Math|Transform|BreakTransform _returnvalue))
  (bind _output_get (LocalVariables|SetGroundSpawnPos (+ (* (LocalVariables|GetPlaneSizeScale) (Math|Vector|MakeVector (.X (Math|Vector|BreakVector (Transformation|GetWorldScale (Variables|Default|GetPlane)))) 0.0 0.0)) _location)))
  (Game|SpawnActorfromClass "BP_Ground_C" (Math|Transform|MakeTransform _output_get _rotation _scale) "Undefined" 0 0))

(fn ItemsSpawn
  (bind _spawnpoints (Variables|Default|GetSpawnPoints))
  (Utilities|Array|Shuffle _spawnpoints)
  (for _index (range 0 (Math|Random|RandomIntegerinRange 0 2))
    (Game|SpawnActorfromClass "/Game/Cube/BP_Obstacle.BP_Obstacle_C" (Math|Transform|MakeTransform (+ "0,0,100.000000" (.Location (Math|Transform|BreakTransform (Utilities|Array|Get(acopy) _spawnpoints _index)))) (.Rotation (Math|Transform|BreakTransform (Utilities|Array|Get(acopy) _spawnpoints _index))) (.Scale (Math|Transform|BreakTransform (Utilities|Array|Get(acopy) _spawnpoints _index)))) "AdjustIfPossibleButAlwaysSpawn" 0 0)))

(fn SetSpawnPoints
  (Variables|Default|SetSpawnPoints (Utilities|Array|MakeArray (Transformation|GetWorldTransform (Variables|Default|GetArrow)) (Transformation|GetWorldTransform (Variables|Default|GetArrow1)) (Transformation|GetWorldTransform (Variables|Default|GetArrow2)) (Transformation|GetWorldTransform (Variables|Default|GetArrow3)) (Transformation|GetWorldTransform (Variables|Default|GetArrow4)) (Transformation|GetWorldTransform (Variables|Default|GetArrow7)) (Transformation|GetWorldTransform (Variables|Default|GetArrow8)) (Transformation|GetWorldTransform (Variables|Default|GetArrow5)) (Transformation|GetWorldTransform (Variables|Default|GetArrow6)))))