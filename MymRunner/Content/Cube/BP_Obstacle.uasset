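; BP_Obstacle is an obstacle actor that removes itself once BP_Character has moved far enough past it.
; A looping one-second timer, started on BeginPlay, runs DestroyTooFarObstacle.
; That function finds the character with GetActorOfClass, compares both Cube components' world X positions, and destroys the obstacle when the character leads by more than a fixed distance.
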(event Custom|Event%20DestroyTooFarObstacle
  (CallFunction|DestroyTooFarObstacle))

(event EventBeginPlay
  (Utilities|Time|SetTimerbyEvent (delegate Custom|Event%20DestroyTooFarObstacle) 1.0 true))

(fn ConstructionScript)

(fn DestroyTooFarObstacle
  (bind _returnvalue (Actor|GetActorOfClass "/Game/Cube/BP_Character.BP_Character_C"))
  (if (> (- (.x (Transformation|GetWorldLocation (Variables|/Game/Cube/BP_Character.BP_Character_C|GetCube _returnvalue))) (.x (Transformation|GetWorldLocation (Variables|Default|GetCube)))) 2e+03)
    (Actor|DestroyActor)))