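; Player character for a cube game, driven by physics impulses on a Cube component for side movement and jumping.
; The move axis adds scaled lateral impulses while CanMove is true, and Space adds an upward impulse, then clears CanJump.
; Cube hits on "ground" tags restore jumping, while "obstacle" tags disable side movement.
; Forward velocity logic is disconnected, and SpawnObstacle and the BeginPlay branch are empty.
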(event OnComponentHit(Cube)
  (params (HitComponent :type Primitive%20Component%20Object%20Reference) (OtherActor :type Actor%20Object%20Reference) (OtherComp :type Primitive%20Component%20Object%20Reference) (NormalImpulse :type Vector :default "0, 0, 0") (Hit :type Hit%20Result%20Structure%20%28by%20ref%29))
  (Utilities|FlowControl|Sequence
    (:then_0
      (if (Actor|ActorHasTag OtherActor "obstacle")
        (Variables|Default|SetcanMove false)))
    (:then_1
      (if (Actor|ActorHasTag OtherActor "ground")
        (Variables|Default|SetcanJump true)))))

(event EventBeginPlay
  (if (Variables|Default|GetcanMove)
    _))

(event Input|AxisEvents|InputAxisMoveRight/Left
  (params (AxisValue :type Float%20%28single-precision%29))
  (if (Variables|Default|GetcanMove)
    (Physics|AddImpulse (Variables|Default|GetCube) (Math|Vector|MakeVector 0.0 (* AxisValue (Variables|Default|GetMoveRight/LeftForce)) 0.0) "None" true)))

(event Input|KeyboardEvents|SpaceBar
  (params (Key :type Key%20Structure :default "None"))
  (:Pressed
    (if (Variables|Default|GetcanJump)
      (Physics|AddImpulse (Variables|Default|GetCube) "0, 0,1000.000000" "None" true)
      (Variables|Default|SetcanJump false))))

(fn ConstructionScript)

(fn SpawnObstacle)